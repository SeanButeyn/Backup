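; PC_Camera is a player-side Blueprint that adds creeps or towers on releasing NumPad One, chosen by the Rolol switch.
; AddCreep and AddTower switch on Rolol again, either growing their array and NumAlive or spawning MyCreep or MyTower at a Spawner transform.
; The array adds have no input, and the Spawner casts never execute.
; AddTower is only called at Rolol 2, which it does not handle.
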(event EventTick
  (params (DeltaSeconds :type Float%20%28single-precision%29)))

(event Input|KeyboardEvents|NumPadOne
  (params (Key :type Key%20Structure :default "AnyKey"))
  (:Released
    (switch int (Variables|Default|GetRolol)
      (:0
        (CallFunction|AddCreep :!label _label))
      (:1
        (goto _label))
      (:2
        (CallFunction|AddTower)))))

(fn ConstructionScript)

(fn AddCreep
  (switch int (Variables|Default|GetRolol)
    (:0
      (Utilities|Array|Add (Variables|Default|Getarry_creep) 0)
      (Math|Integer|IncrementInt (Variables|Default|GetnumAlive)))
    (:1
      (Game|SpawnActorfromClass "/Game/MyCreep.MyCreep_C" (Transformation|GetActorTransform (stale _asspawner)) "Undefined" 0 0))))

(fn AddTower
  (switch int (Variables|Default|GetRolol)
    (:0
      (Utilities|Array|Add (Variables|Default|Getarry_towers) 0)
      (Math|Integer|IncrementInt (Variables|Default|GetnumAlive)))
    (:1
      (Game|SpawnActorfromClass "/Game/MyTower.MyTower_C" (Transformation|GetActorTransform (stale _asspawner)) "Undefined" 0 0))))